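; Mordhau equipment spawner that acts as a walk-over bomb ammo pickup, granting one charge to an overlapping character's carried bomb or big bomb when below max.
; Pickup clears the display and starts a cooldown, which Tick counts down before restocking.
; Restocking briefly spawns the equipment class to copy its randomly customized mesh and materials, adding shine.
; Tick also updates availability and toggles the widget by camera distance with hysteresis.
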(event `self.ReceiveBeginPlay`
  (`self.InitDisplay`))

(event `self.ReceiveTick`
  (params (DeltaSeconds :type "Float (single-precision)"))
  (bind _cooldown_function (`self.Cooldown_Function`))
  (`|ExecutionSequence`
    (:`then_0`
      (if (> _cooldown_function 0.0)
        (set `self.Cooldown_Function` (- _cooldown_function DeltaSeconds))
        (goto _label :!via `Reset`)
        (else
          (`/Engine/EditorBlueprintResources/StandardMacros.DoOnce` false :!label _label
            (:`Completed`
              (`self.RestockDisplay`))))))
    (:`then_1`
      (`self.UpdateVisuals`))))

(event `self.ReceiveActorBeginOverlap`
  (params (OtherActor :type "Actor Object Reference"))
  (bind _asbp_mordhau_character (cast `/Game/Mordhau/Blueprints/Characters/BP_MordhauCharacter` OtherActor))
  (if (`self.CanRestock` _asbp_mordhau_character)
    (`self.SpawnItem` _asbp_mordhau_character)
    (set `self.Cooldown_Function` (`self.Cooldown`))
    (`self.ClearDisplay`)))

(event `InitializeDisplay_EditorOnly`
  (`self.RestockDisplay`))

(fn `CanInteract`
  (params (Character :type "MordhauCharacter Object Reference"))
  (returns (ReturnValue :type Boolean))
  (return false))

(fn `CanRestock`
  (params (Character :type "/Game/Mordhau/Blueprints/Characters/BP_MordhauCharacter Object Reference"))
  (returns (ReturnValue :type Boolean))
  (bind _equipmentclass (`self.EquipmentClass`))
  (if (not (`self.IsOnCooldown`))
    (`/Engine/EditorBlueprintResources/StandardMacros.IsValid` Character
      (:`Is Valid`
        (if (`KismetSystemLibrary.IsValidClass` _equipmentclass)
          (if (== _equipmentclass "/MordhauGlass/BP_Bomb_Big.BP_Bomb_Big_C")
            (bind _asbp_bomb_big (cast `/MordhauGlass/BP_Bomb_Big` (`|GetArrayItem` (`MordhauCharacter.Equipment` Character) 2))
              (:`then`
                (if (>= (`MordhauEquipment.GetAmmo` _asbp_bomb_big) (`MordhauEquipment.GetCurrentMaxAmmo` _asbp_bomb_big))
                  _
                  (else
                    (return true))))
              (:`CastFailed`
                _))
            (else
              (bind _asbp_bomb (cast `/MordhauGlass/BP_Bomb` (`|GetArrayItem` (`MordhauCharacter.Equipment` Character) 1))
                (:`then`
                  (if (>= (`MordhauEquipment.GetAmmo` _asbp_bomb) (`MordhauEquipment.GetCurrentMaxAmmo` _asbp_bomb))
                    _
                    (else
                      (return true))))
                (:`CastFailed`
                  _))))))
      (:`Is Not Valid`
        _)))
  (return false))

(fn `ClearDisplay`
  (bind _lodskeletalmesh (`self.LODSkeletalMesh`))
  (`/Engine/EditorBlueprintResources/StandardMacros.IsValid` (`SkinnedMeshComponent.SkeletalMesh` _lodskeletalmesh)
    (:`Is Valid`
      (`SkinnedMeshComponent.SetSkinnedAssetAndUpdate` _lodskeletalmesh null true)
      (`StaticMeshComponent.SetStaticMesh` (`self.StaticMesh`) null))))

(fn `InitDisplay`
  (if (`KismetSystemLibrary.IsValidClass` (`self.EquipmentClass`))
    (`|ExecutionSequence`
      (:`then_0`
        (`self.RestockDisplay`))
      (:`then_1`
        (bind _returnvalue (`AddComponent|NODE_AddMordhauWidgetComponent-0` :`RelativeTransform` (`KismetMathLibrary.MakeTransform` (`SceneComponent.RelativeLocation` (`self.Scene`)))))
        (set `self.Widget` _returnvalue))
      (:`then_2`
        (`self.SetAvailability` false)
        (set `self.Initialized` true)))))

(fn `IsOnCooldown`
  (returns (ReturnValue :type Boolean))
  (return (> (`self.Cooldown_Function`) 0.0)))

(fn `OnRep_Cooldown`)

(fn `RestockDisplay`
  (bind _lodskeletalmesh (`self.LODSkeletalMesh`))
  (bind _equipmentclass (`self.EquipmentClass`))
  (if (`KismetSystemLibrary.IsValidClass` _equipmentclass)
    (`StaticMeshComponent.SetStaticMesh` (`self.StaticMesh`) null)
    (`|ExecutionSequence`
      (:`then_0`
        (bind _returnvalue (`|SpawnActorFromClass` _equipmentclass (`self.GetTransform`) "Undefined" "OverrideRootScale" null null))
        (bind _asmordhau_equipment (cast `MordhauEquipment` _returnvalue))
        (set `self.Name` (`MordhauEquipment.EquipmentName` _asmordhau_equipment))
        (set `MordhauEquipment.bForceInstantMeshUpdate` true _asmordhau_equipment)
        (bind _returnvalue_2 (`MordhauEquipment.GetRandomCustomization` _asmordhau_equipment true))
        (`MordhauEquipment.AssignCustomization` _asmordhau_equipment _returnvalue_2 0 0 0)
        (bind _skeletalmeshcomponent (`MordhauEquipment.SkeletalMeshComponent` _asmordhau_equipment))
        (`SkinnedMeshComponent.SetSkinnedAssetAndUpdate` _lodskeletalmesh (`SkinnedMeshComponent.SkeletalMesh` _skeletalmeshcomponent) true)
        (`SkinnedMeshComponent.SetPhysicsAsset` _lodskeletalmesh (`MordhauEquipment.PhysicsAsset` _asmordhau_equipment) false)
        (for _index (range (`PrimitiveComponent.GetNumMaterials` _skeletalmeshcomponent))
          (bind _returnvalue_3 (`PrimitiveComponent.GetMaterial` _skeletalmeshcomponent _index))
          (`PrimitiveComponent.SetMaterial` _lodskeletalmesh _index _returnvalue_3)
          (bind _asmaterial_instance_dynamic (cast `MaterialInstanceDynamic` _returnvalue_3))
          (`MaterialInstanceDynamic.SetScalarParameterValue` _asmaterial_instance_dynamic "ShineIntensity" 1.0)))
      (:`then_1`
        (`self.K2_DestroyActor` _returnvalue)))))

(fn `SetAvailability`
  (params (NewAvailable :type Boolean))
  (set `self.IsAvailable` NewAvailable))

(fn `SpawnItem`
  (params (Character :type "/Game/Mordhau/Blueprints/Characters/BP_MordhauCharacter Object Reference"))
  (locals (Emblem :type Integer) (EmblemColor1 :type Byte) (EmblemColor2 :type Byte) (Customization :type "EquipmentCustomization Structure"))
  (bind _equipmentclass (`self.EquipmentClass`))
  (bind _equipment (`MordhauCharacter.Equipment` Character))
  (if (`KismetSystemLibrary.IsValidClass` _equipmentclass)
    (if (== _equipmentclass "/MordhauGlass/BP_Bomb_Big.BP_Bomb_Big_C")
      (bind _asbp_bomb_big (cast `/MordhauGlass/BP_Bomb_Big` (`|GetArrayItem` _equipment 2)))
      (`MordhauEquipment.SetAmmo` _asbp_bomb_big (+ (`MordhauEquipment.GetAmmo` _asbp_bomb_big) 1))
      (else
        (bind _asbp_bomb (cast `/MordhauGlass/BP_Bomb` (`|GetArrayItem` _equipment 1)))
        (`MordhauEquipment.SetAmmo` _asbp_bomb (+ (`MordhauEquipment.GetAmmo` _asbp_bomb) 1))))))

(fn `UpdateVisuals`
  (bind _returnvalue (`KismetMathLibrary.VSize` (- (`self.K2_GetActorLocation`) (`PlayerCameraManager.GetCameraLocation` (`GameplayStatics.GetPlayerCameraManager` 0)))))
  (`|ExecutionSequence`
    (:`then_0`
      (if (not (`self.Initialized`))
        (`self.InitDisplay`)))
    (:`then_1`
      (`self.SetAvailability` (not (`self.IsOnCooldown`))))
    (:`then_2`
      (if (!= (`MordhauWidgetComponent.OverrideVisible` (`self.Widget`)) 0)
        (if (not (< _returnvalue (+ 800.0 25.0)))
          (set `MordhauWidgetComponent.OverrideVisible` 0 (`self.Widget`)))
        (elif (< _returnvalue 800.0)
          (set `MordhauWidgetComponent.OverrideVisible` -1 (`self.Widget`)))))))

(fn `UserConstructionScript`
  (`parent.UserConstructionScript`))