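; Character Blueprint variant that starts with a fixed loadout of a glass sword and two bomb types.
; The first time a profile is assigned, it force-drops and destroys existing equipment, then spawns, randomly customizes and picks up the new items, switching to the sword.
; An empty GiveFists function supplies no fists.
; A pickup-counter RepNotify plays a lift sound when cosmetic events can execute.
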(event `self.ReceiveBeginPlay`
  (`parent.ReceiveBeginPlay`))

(event `self.OnPostProfileAssigned`
  (bind _returnvalue (`self.GetTransform`))
  (`parent.OnPostProfileAssigned`)
  (`/Engine/EditorBlueprintResources/StandardMacros.DoOnce` false
    (:`Completed`
      (for _array_element (`self.Equipment`)
        (`/Engine/EditorBlueprintResources/StandardMacros.IsValid` _array_element
          (:`Is Valid`
            (bind _returnvalue_2 (`self.DropEquipment` _array_element true))
            (`self.K2_DestroyActor` _returnvalue_2))))
      (`|ExecutionSequence`
        (:`then_0`
          (bind _returnvalue_3 (`|SpawnActorFromClass` "/MordhauGlass/BP_GlassSword.BP_GlassSword_C" _returnvalue "Undefined" "OverrideRootScale" null null))
          (bind _returnvalue_4 (`MordhauEquipment.GetRandomCustomization` _returnvalue_3 false))
          (`MordhauEquipment.AssignCustomization` _returnvalue_3 _returnvalue_4 0 0 0)
          (`self.PickUp` _returnvalue_3 0)
          (`self.SwitchEquipment` _returnvalue_3))
        (:`then_1`
          (bind _returnvalue_5 (`|SpawnActorFromClass` "/MordhauGlass/BP_Bomb.BP_Bomb_C" _returnvalue "Undefined" "OverrideRootScale" null null))
          (bind _returnvalue_6 (`MordhauEquipment.GetRandomCustomization` _returnvalue_5 false))
          (`MordhauEquipment.AssignCustomization` _returnvalue_5 _returnvalue_6 0 0 0)
          (`self.PickUp` _returnvalue_5 1))
        (:`then_2`
          (bind _returnvalue_7 (`|SpawnActorFromClass` "/MordhauGlass/BP_Bomb_Big.BP_Bomb_Big_C" _returnvalue "Undefined" "OverrideRootScale" null null))
          (bind _returnvalue_8 (`MordhauEquipment.GetRandomCustomization` _returnvalue_7 false))
          (`MordhauEquipment.AssignCustomization` _returnvalue_7 _returnvalue_8 0 0 0)
          (`self.PickUp` _returnvalue_7 1))))))

(fn `GiveFists`)

(fn `OnRep_PickupCounter`
  (`/Engine/EditorBlueprintResources/StandardMacros.Can Execute Cosmetic Events`
    (:`True`
      (`GameplayStatics.PlaySound2D` "/Game/Mordhau/Audio/Cues/Footsteps/SC_HumanLift.SC_HumanLift" 1.0 1.0 0.0 null null))))

(fn `UserConstructionScript`
  (`parent.UserConstructionScript`))