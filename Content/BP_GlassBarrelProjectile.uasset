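; Explosive glass barrel projectile that detonates on a fuse after being fired, damaging nearby targets and destroying platform actors.
; On firing, it reads the remaining OnLoadedChanged_Timer time from its BP_GlassBarrelExplosive creator and delays by that amount.
; A multi-sphere trace then marks hit BP_PlatformActors destroyed and gates the radial falloff damage.
; Sound, particles and camera shake play regardless, then the actor hides and destroys itself.
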(event `self.ProcessProjectileHit`
  (params (bIsBlocking :type Boolean) (Hit :type "HitResult Structure (by ref)"))
  (`parent.ProcessProjectileHit` bIsBlocking Hit))

(event `CustomEvent_0`
  (bind _returnvalue (`self.GetProjectileCreator`))
  (`KismetSystemLibrary.PrintString` (`KismetSystemLibrary.GetDisplayName` _returnvalue))
  (bind _asbp_glass_barrel_explosive (cast `/MordhauGlass/BP_GlassBarrelExplosive` _returnvalue))
  (set `self.Timer Remaining` (`KismetSystemLibrary.K2_GetTimerRemainingTime` _asbp_glass_barrel_explosive "OnLoadedChanged_Timer")))

(event `self.OnProjectileHit`
  (params (HitLocation :type "Vector Structure") (HitNormal :type "Vector Structure") (BounceForce :type "Float (single-precision)") (Surface :type Byte) (bHasHitWorld :type Boolean) (bHasStopped :type Boolean))
  (`parent.OnProjectileHit` HitLocation HitNormal BounceForce Surface bHasHitWorld bHasStopped))

(event `self.OnProjectileFired`
  (bind _char (`self.Char`))
  (bind _timer_remaining (`self.Timer Remaining`))
  (bind _returnvalue (`SceneComponent.K2_GetComponentLocation` (`self.SkeletalMeshComponent`)))
  (bind _returnvalue_2 (+ _returnvalue (0.0 0.0 300.0)))
  (`self.CustomEvent_0`)
  (`parent.OnProjectileFired`)
  (set `self.RagdollForceMultiplier` 21.0)
  (`KismetSystemLibrary.PrintString` (`KismetStringLibrary.Conv_DoubleToString` _timer_remaining))
  (`KismetSystemLibrary.Delay` _timer_remaining)
  (`|ExecutionSequence`
    (:`then_0`
      (bind (_outhits _returnvalue_3) (`KismetSystemLibrary.SphereTraceMultiForObjects` :`Start` _returnvalue_2 :`End` (* _returnvalue_2 10.0) :`Radius` 400.0 :`ObjectTypes` (`|MakeArray` "ObjectTypeQuery1" "ObjectTypeQuery2" :!type "EObjectTypeQuery Enum") :`bTraceComplex` true :`DrawDebugType` "ForDuration"))
      (if _returnvalue_3
        (for _array_element _outhits
          (bind _asbp_platform_actor (cast `/MordhauGlass/BP_PlatformActor` (`.HitActor` (`GameplayStatics.BreakHitResult` _array_element))))
          (`/MordhauGlass/BP_PlatformActor.SetDestroyed` _asbp_platform_actor))
        (`MordhauUtilityLibrary.MordhauApplyRadialDamageWithFalloff` :`BaseDamage` 300.0 :`MinimumDamage` 50.0 :`Origin` _returnvalue :`DamageInnerRadius` 250.0 :`DamageOuterRadius` 400.0 :`DamageFalloff` 1.0 :`DamageCauser` _char :`InstigatedByController` (`AdvancedCharacter.GetControllerIncludingVehicle` _char))
        (else
          (`KismetSystemLibrary.PrintString` "NO SPHERE TRACE"))))
    (:`then_1`
      (`GameplayStatics.SpawnSoundAttached` "/Game/Mordhau/Audio/Cues/Projectiles/ExplosiveBarrel/SC_ExplosionBarrel2.SC_ExplosionBarrel2" (`self.SkeletalMeshComponent`) "None" (0.0 0.0 0.0) (struct) "KeepRelativeOffset" false 1.15 1.0 0.0 null null))
    (:`then_2`
      (`GameplayStatics.SpawnEmitterAtLocation` "/Game/StarterContent/Particles/KegBreaking.KegBreaking" (`SceneComponent.K2_GetComponentLocation` (`self.SkeletalMeshComponent`)))
      (`GameplayStatics.SpawnEmitterAtLocation` "/MordhauGlass/Particle/GlassExplosion.GlassExplosion" (`SceneComponent.K2_GetComponentLocation` (`self.SkeletalMeshComponent`)) (struct) (0.75 0.75 0.75))
      (`GameplayStatics.SpawnEmitterAtLocation` "/Game/Mordhau/Particles/Fire/Particles/Explosion/Fire_Exp_04_BlackFireBomb.Fire_Exp_04_BlackFireBomb" (`SceneComponent.K2_GetComponentLocation` (`self.SkeletalMeshComponent`)) (struct) (2.5 2.5 2.5)))
    (:`then_3`
      (`GameplayStatics.PlayWorldCameraShake` "/Game/Mordhau/Blueprints/CameraShakes/ExplosionShake.ExplosionShake_C" _returnvalue 1.0 20000.0 10.0 true))
    (:`then_4`
      (`self.SetActorHiddenInGame` true)
      (`KismetSystemLibrary.Delay` 0.3)
      (`self.K2_DestroyActor`))))

(fn `UserConstructionScript`
  (`parent.UserConstructionScript`))