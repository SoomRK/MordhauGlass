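; Breakable glass floor platform that shatters when hit by a bomb projectile or glass sword, or damaged by a player holding a glass sword in the right hand.
; A DoOnce-gated SetDestroyed hides the floor, disables its collision, and plays a geometry cache shatter with sound and effects.
; Reset restores the floor and re-arms the DoOnce.
; BeginPlay assigns the damageable component and a dynamic glass material.
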(event `SetDestroyed`
  (bind _geometrycache (`self.GeometryCache`))
  (bind _floor_400x400 (`self.Floor_400x400`))
  (`/Engine/EditorBlueprintResources/StandardMacros.DoOnce` false :!label _label
    (:`Completed`
      (`ActorComponent.Activate` (`self.GlassBreakBigObject06_Cue`) true)
      (`PrimitiveComponent.SetCollisionEnabled` _floor_400x400 "NoCollision")
      (`SceneComponent.SetVisibility` _floor_400x400 false false)
      (`SceneComponent.SetVisibility` (`self.GeometryCache`) true false)
      (`ActorComponent.Activate` _geometrycache true)
      (`GeometryCacheComponent.PlayFromStart` _geometrycache)
      (`ActorComponent.Activate` (`self.PlankExplosionHuge`) true)
      (`ActorComponent.Activate` (`self.NS_Glass`) true))))

(event `self.ReceiveHit`
  (params (MyComp :type "PrimitiveComponent Object Reference") (Other :type "Actor Object Reference") (OtherComp :type "PrimitiveComponent Object Reference") (bSelfMoved :type Boolean) (HitLocation :type "Vector Structure") (HitNormal :type "Vector Structure") (NormalImpulse :type "Vector Structure") (Hit :type "HitResult Structure (by ref)"))
  (cast `/MordhauGlass/BP_BombProjectile` Other
    (:`then`
      (`self.SetDestroyed`))
    (:`CastFailed`
      (cast `/MordhauGlass/BP_GlassSword` Other)
      (`self.SetDestroyed`))))

(event `self.ReceiveAnyDamage`
  (params (Damage :type "Float (single-precision)") (DamageType :type "DamageType Object Reference") (InstigatedBy :type "Controller Object Reference") (DamageCauser :type "Actor Object Reference"))
  (bind _asbp_mordhau_player_controller (cast `/Game/Mordhau/Blueprints/BP_MordhauPlayerController` InstigatedBy))
  (bind _returnvalue (`MordhauPlayerController.GetControlledMordhauCharacter` _asbp_mordhau_player_controller true))
  (`/Engine/EditorBlueprintResources/StandardMacros.IsValid` _returnvalue
    (:`Is Valid`
      (cast `/MordhauGlass/BP_GlassSword` (`MordhauCharacter.RightHandEquipment` _returnvalue))
      (`self.SetDestroyed`))))

(event `self.ReceiveBeginPlay`
  (bind _floor_400x400 (`self.Floor_400x400`))
  (set `self.DamageableComponent` (`self.Damageable`))
  (bind _returnvalue (`PrimitiveComponent.CreateDynamicMaterialInstance` _floor_400x400 0 "/MordhauGlass/Materials/MI_Glass_1.MI_Glass_1" "None"))
  (`PrimitiveComponent.SetMaterial` _floor_400x400 0 _returnvalue))

(event `Reset`
  (bind _floor_400x400 (`self.Floor_400x400`))
  (`SceneComponent.SetVisibility` (`self.GeometryCache`) false false)
  (`PrimitiveComponent.SetCollisionEnabled` _floor_400x400 "QueryAndPhysics")
  (`SceneComponent.SetVisibility` _floor_400x400 true true)
  (goto _label :!via `Reset`))

(fn `UserConstructionScript`)