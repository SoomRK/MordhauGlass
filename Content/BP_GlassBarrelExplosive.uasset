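; Throwable explosive glass barrel for Mordhau that lights a timed fuse with sparks and sound when its loaded state changes.
; If the timer expires, it destroys traced platform actors, applies radial damage only on a trace hit, plays effects, then removes itself.
; Throwing hands owner and remaining fuse time to BP_GlassBarrelProjectile and clears the local timer.
; Its kills randomly dismember victims with distance-scaled force.
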(event `self.OnUsedToKillOther`
  (params (Character :type "AdvancedCharacter Object Reference") (Type :type "EMordhauDamageType Enum" :default "Generic") (SubType :type Byte) (Bone :type Name) (Point :type "Vector Structure") (Source :type "Actor Object Reference"))
  (bind _killedchar (`self.KilledChar`))
  (bind _returnvalue (- (`SceneComponent.K2_GetComponentLocation` (`self.SkeletalMeshComponent`)) (`SceneComponent.K2_GetComponentLocation` (`Character.CapsuleComponent` _killedchar))))
  ;[1 1 1 1 100] Explosion Dismember
  (`parent.OnUsedToKillOther` Character Type SubType Bone Point Source)
  (bind _asmordhau_character (cast `MordhauCharacter` Character))
  (set `self.KilledChar` _asmordhau_character)
  (for _array_element (`|MakeArray` "head" "RightArm" "RightForearm" "RightHand" "LeftArm" "LeftForearm" "LeftHand" "RightUpLeg" "RightLeg" "RightFoot" "LeftUpLeg" "LeftLeg" "LeftFoot" :!type "Name")
    (if (`KismetMathLibrary.RandomBoolWithWeight` 0.5)
      (`MordhauCharacter.QueueDismember` _killedchar _array_element false false (`KismetMathLibrary.ClampVectorSize` (/ (* (`KismetMathLibrary.Normal` _returnvalue) (- 600.0 (`KismetMathLibrary.VSize` _returnvalue))) 10.0) 1.0 800.0) self))))

(event `self.OnLoadedChanged`
  (`parent.OnLoadedChanged`)
  (`ActorComponent.Activate` (`self.P_ExplosiveSpark`) true)
  (`ActorComponent.Activate` (`self.SC_ExplosiveBarrelFuseThrowable`) true)
  (bind _returnvalue (`KismetSystemLibrary.K2_SetTimerDelegate` (`|CreateDelegate` :!event `OnLoadedChanged_Timer`) 6.0))
  (set `self.NewVar_0` _returnvalue))

(event `self.ReceiveDestroyed`
  (bind _p_explosivespark (`self.P_ExplosiveSpark`))
  (`parent.ReceiveDestroyed`)
  (`ActorComponent.Deactivate` _p_explosivespark)
  (`ActorComponent.Deactivate` (`self.SC_ExplosiveBarrelFuseThrowable`))
  (`SceneComponent.SetHiddenInGame` _p_explosivespark true true)
  (`SceneComponent.SetHiddenInGame` (`self.SC_ExplosiveBarrelFuseThrowable`) true true))

(event `self.OnEquipped`
  (params (Character :type "MordhauCharacter Object Reference"))
  (set `self.StoredOwner` Character)
  (`parent.OnEquipped` Character))

(event `OnLoadedChanged_Timer`
  (bind _storedowner (`self.StoredOwner`))
  (bind _returnvalue (`SceneComponent.K2_GetComponentLocation` (`self.SkeletalMeshComponent`)))
  (bind _returnvalue_2 (+ _returnvalue (0.0 0.0 300.0)))
  (`KismetSystemLibrary.PrintString` "OnLoadedChanged_Timer")
  (`|ExecutionSequence`
    (:`then_0`
      (bind (_outhits _returnvalue_3) (`KismetSystemLibrary.SphereTraceMultiForObjects` :`Start` _returnvalue_2 :`End` (* _returnvalue_2 10.0) :`Radius` 400.0 :`ObjectTypes` (`|MakeArray` "ObjectTypeQuery1" "ObjectTypeQuery2" :!type "EObjectTypeQuery Enum") :`bTraceComplex` true :`DrawDebugType` "ForDuration"))
      (if _returnvalue_3
        (for _array_element _outhits
          (bind _asbp_platform_actor (cast `/MordhauGlass/BP_PlatformActor` (`.HitActor` (`GameplayStatics.BreakHitResult` _array_element))))
          (`/MordhauGlass/BP_PlatformActor.SetDestroyed` _asbp_platform_actor))
        (`MordhauUtilityLibrary.MordhauApplyRadialDamageWithFalloff` :`BaseDamage` 300.0 :`MinimumDamage` 50.0 :`BaseStructureDamage` 0.0 :`Origin` _returnvalue :`DamageInnerRadius` 250.0 :`DamageOuterRadius` 400.0 :`DamageFalloff` 1.0 :`DamageCauser` _storedowner :`InstigatedByController` (`AdvancedCharacter.GetControllerIncludingVehicle` _storedowner))
        (else
          (`KismetSystemLibrary.PrintString` "NO SPHERE TRACE"))))
    (:`then_1`
      (`GameplayStatics.SpawnSoundAttached` "/Game/Mordhau/Audio/Cues/Projectiles/ExplosiveBarrel/SC_ExplosionBarrel2.SC_ExplosionBarrel2" (`self.SkeletalMeshComponent`) "None" (0.0 0.0 0.0) (struct) "KeepRelativeOffset" false 1.15 1.0 0.0 null null))
    (:`then_2`
      (`GameplayStatics.SpawnEmitterAtLocation` "/Game/StarterContent/Particles/KegBreaking.KegBreaking" (`SceneComponent.K2_GetComponentLocation` (`self.SkeletalMeshComponent`)))
      (`GameplayStatics.SpawnEmitterAtLocation` "/MordhauGlass/Particle/GlassExplosion.GlassExplosion" (`SceneComponent.K2_GetComponentLocation` (`self.SkeletalMeshComponent`)) (struct) (0.75 0.75 0.75))
      (`GameplayStatics.SpawnEmitterAtLocation` "/Game/Mordhau/Particles/Fire/Particles/Explosion/Fire_Exp_04_BlackFireBomb.Fire_Exp_04_BlackFireBomb" (`SceneComponent.K2_GetComponentLocation` (`self.SkeletalMeshComponent`)) (struct) (2.5 2.5 2.5)))
    (:`then_3`
      (`GameplayStatics.PlayWorldCameraShake` "/Game/Mordhau/Blueprints/CameraShakes/ExplosionShake.ExplosionShake_C" _returnvalue 1.0 20000.0 10.0 true))
    (:`then_4`
      (`self.SetActorHiddenInGame` true)
      (`KismetSystemLibrary.Delay` 0.3)
      (`self.K2_DestroyActor`))))

(event `self.OnAmmoChanged`
  (`parent.OnAmmoChanged`))

(event `InitProjectile`
  (params (NewParam :type "MordhauProjectile Object Reference"))
  (bind _newvar_0 (`self.NewVar_0`))
  (bind _asbp_glass_barrel_projectile (cast `/MordhauGlass/BP_GlassBarrelProjectile` NewParam))
  (bind _output_get (set `/MordhauGlass/BP_GlassBarrelProjectile.Char` (`self.StoredOwner`) _asbp_glass_barrel_projectile))
  (`KismetSystemLibrary.PrintString` (`KismetSystemLibrary.GetDisplayName` _output_get))
  (bind _output_get_2 (set `/MordhauGlass/BP_GlassBarrelProjectile.Timer Remaining` (`KismetSystemLibrary.K2_GetTimerRemainingTimeHandle` _newvar_0) _asbp_glass_barrel_projectile))
  (`KismetSystemLibrary.PrintString` (`KismetStringLibrary.Conv_DoubleToString` _output_get_2))
  (`KismetSystemLibrary.K2_ClearAndInvalidateTimerHandle` _newvar_0))

(event `self.FireProjectile`
  (params (Origin :type "Vector Structure (by ref)") (Orientation :type "Rotator Structure (by ref)") (OwningController :type "Controller Object Reference") (ExpectedDelay :type "Float (single-precision)"))
  (bind _skeletalmeshcomponent (`MordhauProjectile.SkeletalMeshComponent` (`self.CurrentProjectile`)))
  (`parent.FireProjectile` Origin Orientation OwningController ExpectedDelay)
  (`GameplayStatics.SpawnEmitterAttached` "/Game/StarterContent/Particles/P_ExplosiveSpark.P_ExplosiveSpark" _skeletalmeshcomponent "None" (0.0 0.0 0.0) (struct :`Roll` 180.0))
  (`GameplayStatics.SpawnSoundAttached` "/Game/Mordhau/Audio/Cues/Projectiles/ExplosiveBarrel/SC_ExplosiveBarrelFuseThrowable.SC_ExplosiveBarrelFuseThrowable" _skeletalmeshcomponent "None" (0.0 0.0 0.0) (struct) "KeepRelativeOffset" true 1.0 1.0 0.0 null null))

(event `self.AssignCustomizationToProjectile`
  (params (Projectile :type "MordhauProjectile Object Reference"))
  (`parent.AssignCustomizationToProjectile` Projectile)
  (`self.InitProjectile` Projectile))

(fn `OnRequestModeSwitch`
  (params (Character :type "MordhauCharacter Object Reference"))
  (returns (ReturnValue :type Boolean))
  (return false))

(fn `UserConstructionScript`
  (`parent.UserConstructionScript`))