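; BP_GlassGameMode is the game mode for a round-based glass platform game.
; It overrides StartRoundStart to call the parent, then tell BP_GlassGameState to reset the glass platforms.
; StartRound and EndRound only forward to the parent; an older reset path in StartRound is left disconnected.
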(fn `EndRound`
  (params (IsWipe :type Boolean))
  (`parent.EndRound` IsWipe))

(fn `StartRound`
  (`parent.StartRound`))

(fn `StartRoundStart`
  (`parent.StartRoundStart`)
  (bind _asbp_glass_game_state (cast `/MordhauGlass/BP_GlassGameState` (`GameplayStatics.GetGameState`)))
  (`/MordhauGlass/BP_GlassGameState.ResetGlassPlatforms` _asbp_glass_game_state))

(fn `UserConstructionScript`
  (`parent.UserConstructionScript`))