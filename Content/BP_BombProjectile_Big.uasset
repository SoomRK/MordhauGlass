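; Big bomb projectile that explodes shortly after a hit, damaging players and destroying platforms.
; On hit, parent handling runs while a short delay precedes the explosion effect, sound and knockback radial damage that ignores friendlies.
; A sphere trace slightly above the hit point then calls SetDestroyed on each BP_PlatformActor found.
; Debug trace drawing and a no-hit print remain enabled.
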(event `self.OnProjectileHit`
  (params (HitLocation :type "Vector Structure") (HitNormal :type "Vector Structure") (BounceForce :type "Float (single-precision)") (Surface :type Byte) (bHasHitWorld :type Boolean) (bHasStopped :type Boolean))
  (bind _returnvalue (+ HitLocation (0.0 0.0 125.0)))
  (`|ExecutionSequence`
    (:`then_0`
      (`KismetSystemLibrary.Delay` 0.2)
      (`GameplayStatics.SpawnEmitterAtLocation` "/Game/Mordhau/Particles/Fire/Particles/Explosion/Fire_Exp_04_BlackFireBomb.Fire_Exp_04_BlackFireBomb" HitLocation)
      (`GameplayStatics.PlaySoundAtLocation` "/Game/Mordhau/Audio/Cues/Projectiles/Pots/SC_BlackPot_Explode.SC_BlackPot_Explode" HitLocation (struct) 1.0 1.3 0.0 null null null)
      (bind _returnvalue_2 (`self.GetProjectileOwningController`))
      (`MordhauUtilityLibrary.MordhauApplyRadialDamageWithFalloff` :`BaseDamage` 50.0 :`MinimumDamage` 50.0 :`Origin` HitLocation :`DamageInnerRadius` 80.0 :`DamageOuterRadius` 250.0 :`DamageFalloff` 1.0 :`BaseKnockback` 3000.0 :`MinimumKnockback` 3000.0 :`RagdollFallRadius` 100.0 :`DamageCauser` self :`InstigatedByController` _returnvalue_2 :`DamagePreventionChannel` "ECC_Vehicle" :`bIgnoreFriendly` true)
      (bind (_outhits _returnvalue_3) (`KismetSystemLibrary.SphereTraceMultiForObjects` :`Start` _returnvalue :`End` _returnvalue :`Radius` 260.0 :`ObjectTypes` (`|MakeArray` "ObjectTypeQuery1" "ObjectTypeQuery2" :!type "EObjectTypeQuery Enum") :`bTraceComplex` true :`DrawDebugType` "ForDuration"))
      (if _returnvalue_3
        (for _array_element _outhits
          (bind _asbp_platform_actor (cast `/MordhauGlass/BP_PlatformActor` (`.HitActor` (`GameplayStatics.BreakHitResult` _array_element))))
          (`/MordhauGlass/BP_PlatformActor.SetDestroyed` _asbp_platform_actor))
        (else
          (`KismetSystemLibrary.PrintString` "NO SPHERE TRACE"))))
    (:`then_1`
      (`parent.OnProjectileHit` HitLocation HitNormal BounceForce Surface bHasHitWorld bHasStopped))))

(fn `UserConstructionScript`
  (`parent.UserConstructionScript`))